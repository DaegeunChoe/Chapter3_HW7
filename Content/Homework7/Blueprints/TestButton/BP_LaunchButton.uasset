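; BP_LaunchButton is a button that, judging by its name and logic, launches a movement target when triggered.
; It overrides OnTrigger, calling the parent first, then checks that the MyMovement reference is valid.
; It applies a brief instant force, scaled up from the Force variable, through MyMovement and then calls Jump on it.
; The event graph holds only disabled placeholder events.
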(event EventBeginPlay
  (|CallParentFunction) ; This node is disabled and will not be called.\nDrag off pins to build functionality.
)

(event Collision|EventActorBeginOverlap
  (params (OtherActor :type Actor%20Object%20Reference)))

(event EventTick
  (params (DeltaSeconds :type Float%20%28single-precision%29)))

(fn ConstructionScript
  (|CallParentFunction))

(fn OnTrigger
  (|CallParentFunction)
  (bind _my_movement (Variables|Default|GetMy%20Movement)
    (:then
      (Class|MyPhysicsMovement|SetInstantForce _my_movement (* (Variables|Default|GetForce) (Math|Float|MakeLiteralFloat 1e+02)) 0.2)
      (Class|MyCharacterMovement|Jump _my_movement))
    (:else)))