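; BP_StaticFrictionText is a debug text display that shows the player pawn's maximum static friction coefficient.
; On BeginPlay it casts player 0's pawn to MyPawn and caches that pawn and its MyMovement component.
; Each Tick, while the movement component is valid, it formats a label with MaxStaticFrictionCoefficient and writes it to its TextRender component.
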(event EventBeginPlay
  (bind _asmy_pawn (Utilities|Casting|CastToMyPawn (Game|Player|GetPlayerPawn 0)))
  (bind _output_get (Variables|Default|SetMyPawn _asmy_pawn))
  (Variables|Default|SetMy%20Movement (Variables|/Script/Homework7.MyPawn|GetMyMovement _output_get)))

(event EventTick
  (params (DeltaSeconds :type Float%20%28single-precision%29))
  (bind _my_movement (Variables|Default|GetMy%20Movement)
    (:then
      (Rendering|Components|TextRender|SetText (Variables|Default|GetTextRender) (Utilities|Text|FormatText "{label}: {value}" (Variables|Default|GetLabel) (Variables|/Script/Homework7.MyPhysicsMovement|GetMaxStaticFrictionCoefficient _my_movement))))
    (:else)))

(fn ConstructionScript)