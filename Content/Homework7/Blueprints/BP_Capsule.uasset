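; BP_Capsule is a test actor that exercises a MyPhysicsMovement component with a constant push and on-screen debug readouts.
; On BeginPlay it sets an additional force along the Y axis on the component.
; Each Tick it draws the component's net force and velocity as colored debug text above the actor, with both operations guarded by validity checks.
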(event EventTick
  (params (DeltaSeconds :type Float%20%28single-precision%29))
  (bind _myphysicsmovement (Variables|Components|GetMyPhysicsMovement)
    (:then
      (Rendering|Debug|DrawDebugString (+ (Transformation|GetActorLocation) "0.000000,0.000000,100.000000") (Utilities|String|ToString(Vector) (Variables|/Script/Homework7.MyPhysicsMovement|GetNetForce _myphysicsmovement)) 0 "(R=0.064095,G=0.000000,B=1.000000,A=1.000000)")
      (Rendering|Debug|DrawDebugString (+ (Transformation|GetActorLocation) "0.000000,0.000000,80.000000") (Utilities|String|ToString(Vector) (Variables|/Script/Homework7.MyPhysicsMovement|GetVelocity (Variables|Components|GetMyPhysicsMovement))) 0 "(R=0.000000,G=1.000000,B=0.228051,A=1.000000)"))
    (:else)))

(event EventBeginPlay
  (bind _myphysicsmovement (Variables|Components|GetMyPhysicsMovement)
    (:then
      (Class|MyPhysicsMovement|SetAdditionalForce _myphysicsmovement "0.000000,3000.000000,0.000000"))
    (:else)))

(fn ConstructionScript)