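; BP_MyPawn is a pawn Blueprint that displays live debug readouts of its movement state.
; Each tick it checks that MyMovement is valid, then draws that object's NetForce and Velocity as two differently colored debug strings stacked above the actor's location.
; The construction script is empty, and the graphs here only read the movement values without changing them.
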(event EventTick
  (params (DeltaSeconds :type Float%20%28single-precision%29))
  (bind _mymovement (Variables|Default|GetMyMovement)
    (:then
      (Rendering|Debug|DrawDebugString (+ (Transformation|GetActorLocation) "0.000000,0.000000,100.000000") (Utilities|String|ToString(Vector) (Variables|/Script/Homework7.MyPhysicsMovement|GetNetForce _mymovement)) 0 "(R=0.064095,G=0.000000,B=1.000000,A=1.000000)")
      (bind _mymovement_2 (Variables|Default|GetMyMovement)
        (:then
          (Rendering|Debug|DrawDebugString (+ (Transformation|GetActorLocation) "0.000000,0.000000,80.000000") (Utilities|String|ToString(Vector) (Variables|/Script/Homework7.MyPhysicsMovement|GetVelocity _mymovement_2)) 0 "(R=1.000000,G=0.000000,B=0.102203,A=1.000000)"))
        (:else)))
    (:else)))

(fn ConstructionScript)